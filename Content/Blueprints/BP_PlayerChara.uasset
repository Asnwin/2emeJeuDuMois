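; BP_PlayerChara is the player character, handling movement, camera look and projectile shooting.
; Move axes add input along yaw-only control rotation vectors, while look axes feed controller pitch and yaw.
; Shoot spawns BP_Bullet near the mesh, offset and aimed by camera rotation, calls an emitter spawn and sets Fire until release.
; A disconnected camera line-trace remains unused.
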(event EventBeginPlay)

(event Collision|EventActorBeginOverlap
  (params (OtherActor :type Actor%20Object%20Reference)))

(event EventTick
  (params (DeltaSeconds :type Float%20%28single-precision%29)))

(event Input|ActionEvents|InputActionShoot
  (params (Key :type Key%20Structure :default "None"))
  (bind _camera (Variables|Default|GetCamera))
  (bind _returnvalue (Transformation|GetWorldRotation _camera))
  (:Pressed
    (Variables|Default|SetFire true)
    (Game|SpawnActorfromClass "/Game/Blueprints/BP_Bullet.BP_Bullet_C" (Math|Transform|MakeTransform (+ (Transformation|GetWorldLocation (Variables|Character|GetMesh)) (Math|Vector|RotateVector "5.000000,5.000000,5.000000" _returnvalue)) _returnvalue) "AdjustIfPossibleButDontSpawnIfColliding" 0 0)
    (Effects|SpawnEmitteratLocation 0 "0, 0, 0"))
  (:Released
    (Variables|Default|SetFire false)))

(event Input|AxisEvents|InputAxisMoveRightLeft
  (params (AxisValue :type Float%20%28single-precision%29))
  ;[1 1 1] Chara Controller
  (Pawn|Input|AddMovementInput (Math|Vector|GetRightVector (Math|Rotator|MakeRotator 0.0 0.0 (.Yaw (Math|Rotator|BreakRotator (Pawn|GetControlRotation :!class /Script/Engine.Pawn))))) AxisValue false))

(event Input|AxisEvents|InputAxisLookUpDown
  (params (AxisValue :type Float%20%28single-precision%29))
  ;[1 1 1] Camera Controller
  (Pawn|Input|AddControllerPitchInput AxisValue))

(event Input|AxisEvents|InputAxisLookSides
  (params (AxisValue :type Float%20%28single-precision%29))
  ;[1 1 1] Camera Controller
  (Pawn|Input|AddControllerYawInput AxisValue))

(event Input|AxisEvents|InputAxisMoveForward
  (params (AxisValue :type Float%20%28single-precision%29))
  ;[1 1 1] Chara Controller
  (Pawn|Input|AddMovementInput (Math|Vector|GetForwardVector (Math|Rotator|MakeRotator 0.0 0.0 (.Yaw (Math|Rotator|BreakRotator (Pawn|GetControlRotation :!class /Script/Engine.Pawn))))) AxisValue false))

(fn ConstructionScript)